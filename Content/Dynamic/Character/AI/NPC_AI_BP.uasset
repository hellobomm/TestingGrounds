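; NPC AI controller that runs a guard behavior tree and tracks a perceived target for it.
; On BeginPlay it sets up the PatrolData blackboard, starts GuardBehaviour and caches the blackboard component.
; AI perception updates set the enemy actor key when a target is sensed and clear it when sensing fails.
; Actors tagged "enemy" are ignored, so only untagged actors affect that key.
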(event `self.ReceiveBeginPlay`
  (bind _blackboardcomponent (`self.UseBlackboard` "/Game/Dynamic/Character/AI/PatrolData.PatrolData"))
  (`self.RunBehaviorTree` "/Game/Dynamic/Character/AI/GuardBehaviour.GuardBehaviour")
  (set `self.Blackboard_Comp` _blackboardcomponent))

(event `self.AIPerception.OnTargetPerceptionUpdated`
  (params (Actor :type "Actor Object Reference") (Stimulus :type "AIStimulus Structure"))
  (`self.Update Blackboard EnemyKey` Actor Stimulus Actor))

(fn `Update Blackboard EnemyKey`
  (params (ObjectValue :type "Object Object Reference") (AIStimulus :type "AIStimulus Structure (by ref)") (self2 :type "Actor Object Reference"))
  (bind _blackboard_comp (`self.Blackboard_Comp`))
  (bind _enemyactor_key (`self.EnemyActor Key`))
  (if (`self.ActorHasTag` self2 "enemy")
    _
    (elif (`.bSuccessfullySensed` (break `AIStimulus` AIStimulus))
      (`BlackboardComponent.SetValueAsObject` _blackboard_comp _enemyactor_key ObjectValue)
      (else
        (`BlackboardComponent.ClearValue` _blackboard_comp _enemyactor_key)))))

(fn `UserConstructionScript`)