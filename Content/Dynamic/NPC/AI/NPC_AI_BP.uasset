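; AI controller for guard NPCs that aim and shoot at actors they perceive.
; On BeginPlay it sets up the PatrolData blackboard, runs the GuardBehaviour tree and resets the controlled ThirdPersonCharacter's combat flags.
; Perception updates ignore actors tagged "enemy".
; For others, sensing sets the enemy blackboard key and the Aiming and Shooting flags, and losing them clears all three.
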(event `self.ReceiveBeginPlay`
  (bind _blackboardcomponent (`self.UseBlackboard` "/Game/Dynamic/NPC/AI/PatrolData.PatrolData"))
  (`self.RunBehaviorTree` "/Game/Dynamic/NPC/AI/GuardBehaviour.GuardBehaviour")
  (set `self.Blackboard_Comp` _blackboardcomponent)
  (bind _asthird_person_character (cast `/Game/Dynamic/NPC/Behaviour/ThirdPersonCharacter` (`self.K2_GetPawn`)))
  (bind _output_get (set `self.AICharacter` _asthird_person_character))
  (set `/Game/Dynamic/NPC/Behaviour/ThirdPersonCharacter.Aiming` false _output_get)
  (set `/Game/Dynamic/NPC/Behaviour/ThirdPersonCharacter.Shooting` false _output_get))

(event `self.AIPerception.OnTargetPerceptionUpdated`
  (params (Actor :type "Actor Object Reference") (Stimulus :type "AIStimulus Structure"))
  (bind _blackboard_comp (`self.Blackboard_Comp`))
  (bind _enemyactor_key (`self.EnemyActor Key`))
  (bind _aicharacter (`self.AICharacter`))
  (if (`self.ActorHasTag` Actor "enemy")
    _
    (elif (`.bSuccessfullySensed` (break `AIStimulus` Stimulus))
      (`BlackboardComponent.SetValueAsObject` _blackboard_comp _enemyactor_key Actor)
      (set `/Game/Dynamic/NPC/Behaviour/ThirdPersonCharacter.Aiming` true _aicharacter)
      (set `/Game/Dynamic/NPC/Behaviour/ThirdPersonCharacter.Shooting` true _aicharacter)
      (else
        (`BlackboardComponent.ClearValue` _blackboard_comp _enemyactor_key)
        (set `/Game/Dynamic/NPC/Behaviour/ThirdPersonCharacter.Aiming` false _aicharacter)
        (set `/Game/Dynamic/NPC/Behaviour/ThirdPersonCharacter.Shooting` false _aicharacter)))))

(fn `UserConstructionScript`)